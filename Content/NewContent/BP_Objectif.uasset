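; BP_Objectif is an interactable objective that counts as a collectible page for the player.
; On Interact it runs the parent logic, looks up the FirstPersonCharacter with GetActorOfClass, increments that character's Pages counter and destroys itself.
; BeginPlay, overlap, Tick and construction only hold parent calls, so all of its own behavior lives in Interact.
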(event `self.ReceiveActorBeginOverlap`
  (params (OtherActor :type "Actor Object Reference"))
  (`parent.ReceiveActorBeginOverlap` OtherActor))

(event `self.ReceiveTick`
  (params (DeltaSeconds :type "Float (single-precision)"))
  (`parent.ReceiveTick` DeltaSeconds))

(event `/Game/InteractionSystem/IInteractable.interact`
  (`parent.interact`)
  (bind _returnvalue (`GameplayStatics.GetActorOfClass` "/Game/FirstPersonCharacter.FirstPersonCharacter_C"))
  (bind _result (`/Engine/EditorBlueprintResources/StandardMacros.IncrementInt` (`/Game/FirstPersonCharacter.Pages` _returnvalue))
    (:`  `
      (set `/Game/FirstPersonCharacter.Pages` _result _returnvalue)
      (`self.K2_DestroyActor`))))

(fn `UserConstructionScript`
  (`parent.UserConstructionScript`))